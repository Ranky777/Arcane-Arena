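; GA_Dash is a gameplay ability that gives an ArcaneCharacter a short, fast dash.
; On activation it commits the ability, blends out the playing montage and picks the current velocity direction, or actor forward when stationary.
; A brief constant root motion force drives the dash and maintains its velocity on finish.
; The ability ends when the force finishes or a matching delay elapses.
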(event `self.K2_ActivateAbility`
  (bind _returnvalue (`self.GetAvatarActorFromActorInfo`))
  (bind _asarcane_character (cast `ArcaneCharacter` _returnvalue))
  (`self.K2_CommitAbility`)
  (`AnimInstance.Montage_Stop` (`SkeletalMeshComponent.GetAnimInstance` (`Character.Mesh` _asarcane_character)) 0.1 null)
  (bind _returnvalue_2 (`Actor.GetVelocity` _asarcane_character))
  (if (> (`KismetMathLibrary.VSize` _returnvalue_2) 0.01)
    (set `self.CurrentDireaction` (`KismetMathLibrary.Normal` _returnvalue_2))
    (else
      (set `self.CurrentDireaction` (`Actor.GetActorForwardVector` _returnvalue))))
  (`AbilityTask_ApplyRootMotionConstantForce.ApplyRootMotionConstantForce` "None" (`self.CurrentDireaction`) 3000.0 0.15 false null "MaintainLastRootMotionVelocity"
    (:`then`
      (`AbilityTask_WaitDelay.WaitDelay` 0.15
        (:`OnFinish`
          (`self.K2_EndAbility`))))
    (:`OnFinish`
      (`self.K2_EndAbility`))))