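; BP_NetGuardCheatTester is a debug actor that simulates a cheating client to exercise server-side RPC validation on ArcaneCharacter.
; On tick, a non-authority instance watches for the K key on the first player controller.
; When pressed, it fires a burst of HomingBolt homing-attack server RPCs from the local pawn, targeting that pawn itself and aiming ahead of it.
; Debug prints report the send or a failed character cast.
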(event `self.ReceiveTick`
  (params (DeltaSeconds :type "Float (single-precision)"))
  (if (and (not (`self.HasAuthority` self)) (`PlayerController.WasInputKeyJustPressed` (`GameplayStatics.GetPlayerController` 0) "K"))
    (bind _asarcane_character (cast `ArcaneCharacter` (`GameplayStatics.GetPlayerPawn` 0))
      (:`then`
        (`KismetSystemLibrary.PrintString` "NetGuardCheat: K pressed, sending 20 Homing RPCs")
        (for _ (range 20)
          (`ArcaneCharacter.ServerRequestHomingAttack` _asarcane_character (`KismetStringLibrary.Conv_StringToName` "HomingBolt") _asarcane_character (+ (`self.K2_GetActorLocation` _asarcane_character) (* (`self.GetActorForwardVector` _asarcane_character) 1000.0)))))
      (:`CastFailed`
        (`KismetSystemLibrary.PrintString` "NetGuardCheat: pawn is not ArcaneCharacter")))))

(fn `UserConstructionScript`)